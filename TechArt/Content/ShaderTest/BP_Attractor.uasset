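; BP_Attractor is a shader-test actor that publishes its location to the MPC_Attractor material parameter collection and oscillates along world Y during play.
; The Construction Script writes the location, while Tick accumulates time to drive a sine offset on the root without updating the collection.
; The nodes that capture the starting position never run, so motion uses the stored variable values.
; Writes to MPC_Light are also disconnected.
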(event EventBeginPlay)

(event Collision|EventActorBeginOverlap
  (params (OtherActor :type Actor%20Object%20Reference)))

(event EventTick
  (params (DeltaSeconds :type Float%20%28single-precision%29))
  (bind _output_get (Variables|Default|SetNewVar_0 (+ DeltaSeconds (Variables|Default|GetNewVar_0))))
  (Transformation|SetWorldLocation (Variables|Default|GetDefaultSceneRoot) (Math|Vector|MakeVector (Variables|Default|GetNewVar_1) (|((a*(sin(b)))+c) 1e+02 (* _output_get 5.0) (Variables|Default|GetNewVar_2)) (Variables|Default|GetNewVar_3)) false false))

(fn ConstructionScript
  (Utilities|FlowControl|Sequence
    (:then_0
      (Rendering|Material|SetVectorParameterValue "/Game/ShaderTest/MPC_Attractor.MPC_Attractor" "Location" (Math|Conversions|ToLinearColor(Vector) (Transformation|GetWorldLocation (Variables|Default|GetDefaultSceneRoot))) :!class /Script/Engine.KismetMaterialLibrary))))
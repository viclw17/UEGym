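; BP_SSSFaker is a scene capture actor, named as a subsurface scattering fake, that captures a chosen actor along the sun's axis.
; Its construction script limits the SceneCaptureComponent2D to CaptureActor, then points itself opposite SunActor's direction by flipping pitch and roll.
; The rotation updates only on construction, as the event graph is empty.
; Nodes writing light position and color to MPC_Light exist but are disconnected.
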(event EventBeginPlay)

(event Collision|EventActorBeginOverlap
  (params (OtherActor :type Actor%20Object%20Reference)))

(event EventTick
  (params (DeltaSeconds :type Float%20%28single-precision%29)))

(fn ConstructionScript
  (bind _sunactor (Variables|Default|GetSunActor))
  (bind _returnvalue (Transformation|GetActorRotation _sunactor))
  (bind (_roll _pitch _yaw) (Math|Rotator|BreakRotator _returnvalue))
  (Utilities|FlowControl|Sequence
    (:then_1
      (Rendering|SceneCapture|ShowOnlyActorComponents (Variables|Default|GetSceneCaptureComponent2D) (Variables|Default|GetCaptureActor)))
    (:then_2
      (Transformation|SetActorRotation (Math|Rotator|MakeRotator 1.8e+02 (+ _pitch 1.8e+02) _yaw)))))
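; Blueprint function library in the FPP Template for coloring power materials by power type.
; It looks up colors in the DT_FPPT_Colors data table using the enum name as the row, falling back to the "Type_1" row if none matches.
; Setup applies base and emissive colors to a material instance, then calls Update, which scales emissive amount from zero to the type's value by power level.
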(fn GetPowerTypeColors
  (params (Type :type Enum_FPPT_Colors%20Enum :default "NewEnumerator1"))
  (bind _returnvalue (Utilities|GetDataTableRow "/Game/FPPTemplate/Blueprints/Core/DT_FPPT_Colors.DT_FPPT_Colors" (Utilities|String|StringToName (Utilities|String|EnumtoString Type)))
    (:then
      (return _returnvalue))
    (:RowNotFound
      (bind _returnvalue_2 (Utilities|GetDataTableRow "/Game/FPPTemplate/Blueprints/Core/DT_FPPT_Colors.DT_FPPT_Colors" "Type_1")
        (:then
          (return _returnvalue_2))))))

(fn UpdatePowerMaterial
  (params (Material%20Instance :type Material%20Instance%20Dynamic%20Object%20Reference) (Power :type Float%20%28single-precision%29) (Power%20Type :type Enum_FPPT_Colors%20Enum :default "NewEnumerator1"))
  (Rendering|Material|SetScalarParameterValue Material%20Instance "Emissive Amount" (Math|Float|Lerp 0.0 (.EmissiveAmount (Utilities|Struct|BreakStruct_FPPT_Colors (CallFunction|GetPowerTypeColors Power%20Type (LocalVariables|Get__WorldContext)))) Power) :!class /Script/Engine.MaterialInstanceDynamic))

(fn SetupPowerMaterial
  (params (Material%20Instance :type Material%20Instance%20Dynamic%20Object%20Reference) (Power :type Float%20%28single-precision%29) (Power%20Type :type Enum_FPPT_Colors%20Enum :default "NewEnumerator1"))
  (bind ___worldcontext (LocalVariables|Get__WorldContext))
  (bind _type_colors (CallFunction|GetPowerTypeColors Power%20Type ___worldcontext))
  (bind (_basecolor _emissivecolor) (Utilities|Struct|BreakStruct_FPPT_Colors _type_colors))
  (Rendering|Material|SetVectorParameterValue Material%20Instance "Base Color" (Math|Conversions|ToLinearColor(Color) _basecolor) :!class /Script/Engine.MaterialInstanceDynamic)
  (Rendering|Material|SetVectorParameterValue Material%20Instance "Emissive Color" (Math|Conversions|ToLinearColor(Color) _emissivecolor) :!class /Script/Engine.MaterialInstanceDynamic)
  (CallFunction|UpdatePowerMaterial Material%20Instance Power Power%20Type (LocalVariables|Get__WorldContext)))
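; BP_FPPT_CubeActivator is a trigger actor that toggles the active power state of one assigned cube when that cube overlaps it.
; Overlap calls OnPowerUpdate on CubeToChange with its inverted Active value, either every time or once through a DoOnce gate, with optional self-destruction afterwards.
; The construction script passes the cube's power-type color to SetDebugColors, which is empty here, and BeginPlay applies HideInGame to its Cube component.
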(event Custom|Set%20Debug%20Colors
  (params (Color :type Color%20Structure)))

(event EventBeginPlay
  (Development|SetHiddeninGame (Variables|Default|GetCube) (Variables|Default|GetHideInGame) false))

(event EventTick
  (params (DeltaSeconds :type Float%20%28single-precision%29)))

(event Collision|EventActorBeginOverlap
  (params (OtherActor :type Actor%20Object%20Reference))
  (bind _cubetochange (Variables|Default|GetCubeToChange))
  (bind _cubetochange_2 (Variables|Default|GetCubeToChange))
  (if (and (== OtherActor _cubetochange) (Utilities|IsValid _cubetochange))
    (if (Variables|Default|GetDoOnce)
      (Utilities|FlowControl|DoOnce false :!label _label
        (:Completed
          (Utilities|FlowControl|Sequence
            (:then_0
              (Default|OnPowerUpdate _cubetochange_2 (not (Variables|/Game/FPPTemplate/Blueprints/Core/BP_FPPT_Base.BP_FPPT_Base_C|GetActive _cubetochange_2)) false :!label _label_2))
            (:then_1
              (if (Variables|Default|GetDeleteAfterDoOnce?)
                (Actor|DestroyActor))))))
      (else
        (Utilities|FlowControl|Sequence
          (:then_0
            (goto _label Reset))
          (:then_1
            (goto _label_2)))))))

(fn ConstructionScript
  (Utilities|IsValid (Variables|Default|GetCubeToChange)
    (:Is%20Valid
      (CallFunction|SetDebugColors (.BaseColor (Utilities|Struct|BreakStruct_FPPT_Colors (CallFunction|GetPowerTypeColors (Variables|/Game/FPPTemplate/Blueprints/Core/BP_FPPT_Base.BP_FPPT_Base_C|GetPower%20Type (Variables|Default|GetCubeToChange)))))))))
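; Logic gate actor that delays a power signal before passing it on to its target actor.
; While active, Tick counts down the delay and, once it expires, re-fires the power update so the parent class can propagate it.
; Losing power resets the countdown, with DoOnce nodes guarding the one-shot transitions.
; A text render shows the remaining whole seconds, tinted by power type and active state.
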(event EventBeginPlay
  (|CallParentFunction) ; This node is disabled and will not be called.\nDrag off pins to build functionality.
)

(event Collision|EventActorBeginOverlap
  (params (OtherActor :type Actor%20Object%20Reference))
  (|CallParentFunction OtherActor) ; This node is disabled and will not be called.\nDrag off pins to build functionality.
)

(event EventOnPowerUpdate
  (params (New%20Active :type Boolean) (Is%20Forced :type Boolean) (Intial%20Actor :type Actor%20Object%20Reference))
  (Utilities|FlowControl|Sequence
    (:then_0
      (if (and (Math|Boolean|NotEqual(Boolean) New%20Active (Variables|Default|GetActive)) (Variables|Default|GetActive))
        (|CallParentFunction New%20Active Is%20Forced Intial%20Actor :!label _label)
        (elif (CallFunction|GetActiveStatus)
          (goto _label))))
    (:then_1
      (Variables|Default|SetActive New%20Active)
      (if (Variables|Default|GetActive)
        (goto _label_2 Reset)
        (else
          (Utilities|FlowControl|DoOnce false :!label _label_2
            (:Completed
              (Variables|Default|SetCurrentDelay (Math|Conversions|ToFloat(Integer) (Variables|Default|GetDelay)))
              (CallFunction|UpdateText)
              (if (and (Variables|Default|GetActivated%20Timer) (not (Variables|Default|GetActive)))
                (Variables|Default|SetActivated%20Timer false)
                (goto _label)))))))))

(event EventTick
  (params (DeltaSeconds :type Float%20%28single-precision%29))
  (|CallParentFunction DeltaSeconds)
  (if (Variables|Default|GetActive)
    (Variables|Default|SetActivated%20Timer true)
    (if (>= (Variables|Default|GetCurrentDelay) 0.0)
      (Variables|Default|SetCurrentDelay (- (Variables|Default|GetCurrentDelay) DeltaSeconds))
      (CallFunction|UpdateText)
      (goto _label Reset)
      (else
        (Utilities|FlowControl|DoOnce false :!label _label
          (:Completed
            (CallFunction|UpdateText)
            (Default|OnPowerUpdate self (Variables|Default|GetActive) false self)))))))

(event EventRunConstructionScriptsNonGenerative
  (params (Forced :type Boolean))
  (|CallParentFunction false)
  (CallFunction|UpdateText))

(event EventSetupMaterialOwners
  (Rendering|Material|SetMaterial (Variables|Default|GetStaticMesh) 0 (Variables|Default|GetMain%20Power%20Material)))

(event EventOnUpdatePowerFinished
  (params (Forced :type Boolean))
  (CallFunction|UpdatePoweronTarget Forced (Variables|Default|GetTargetActor) false false))

(fn ConstructionScript
  (|CallParentFunction)
  (Variables|Default|SetCurrentDelay (Math|Conversions|ToFloat(Integer) (Variables|Default|GetDelay)))
  (CallFunction|UpdateText))

(fn GetActiveStatus
  (return (<= (Variables|Default|GetCurrentDelay) 0.0)))

(fn UpdateText
  (bind _power_type (Variables|Default|GetPower%20Type))
  (bind _type_colors (CallFunction|GetPowerTypeColors _power_type))
  (bind (_basecolor _emissivecolor) (Utilities|Struct|BreakStruct_FPPT_Colors _type_colors))
  (Rendering|Components|TextRender|SetText (Variables|Default|GetTimerText) (Utilities|Text|ToText(Integer) (Math|Integer|Max(Integer) (Math|Float|Floor (Variables|Default|GetCurrentDelay)))))
  (Rendering|Components|TextRender|SetTextRenderColor (Variables|Default|GetTimerText) (select (Variables|Default|GetActive) _emissivecolor _basecolor)))
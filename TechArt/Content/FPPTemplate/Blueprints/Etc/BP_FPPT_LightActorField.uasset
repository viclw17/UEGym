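; BP_FPPT_LightActorField builds a rectangular field of BP_FPPT_Light actors centered on its own origin.
; Its construction script loops over the Grid X and Y counts, adding a child actor component for each cell, with Grid Z serving as the spacing.
; Each offset subtracts half the field's extent plus half a cell, so the lights sit symmetrically on a flat plane.
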(fn ConstructionScript
  (bind _grid (Variables|Default|GetGrid))
  (bind (_x _y _z) (Utilities|Struct|BreakIntVector _grid))
  (bind _returnvalue (Math|Conversions|ToFloat(Integer) _z))
  (bind _returnvalue_2 (Math|Conversions|ToFloat(Integer) _z))
  (bind _returnvalue_3 (/ _returnvalue_2 2.0))
  (for _index (range 1 _x)
    (for _index_2 (range 1 _y)
      (bind _returnvalue_4 (AddComponent|AddChildActorComponent false (Math|Transform|MakeTransform (- (Math|Vector|MakeVector (* _index _returnvalue) (* _index_2 _returnvalue) 0.0) (+ (/ (Math|Vector|MakeVector (* _x _returnvalue_2) (* _y _returnvalue_2) 0.0) 2.0) (Math|Vector|MakeVector _returnvalue_3 _returnvalue_3 0.0))) "0, 0, 0" "1.000000,1,1")))
      (ChildActorComponent|SetChildActorClass _returnvalue_4 "/Game/FPPTemplate/Blueprints/Etc/BP_FPPT_Light.BP_FPPT_Light_C"))))
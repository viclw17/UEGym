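; BP_FPPT_PowerBlock is a power block actor in the FPP Template that relays power updates to a target actor.
; SetupMaterialOwners applies the main power material to the first slot of its two static meshes.
; When a power update finishes, it calls UpdatePowerOnTarget on TargetActor, passing the Forced flag along.
; BeginPlay, overlap, Tick and the construction script add no logic of their own.
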(event EventBeginPlay
  (|CallParentFunction) ; This node is disabled and will not be called.\nDrag off pins to build functionality.
)

(event Collision|EventActorBeginOverlap
  (params (OtherActor :type Actor%20Object%20Reference))
  (|CallParentFunction OtherActor) ; This node is disabled and will not be called.\nDrag off pins to build functionality.
)

(event EventTick
  (params (DeltaSeconds :type Float%20%28single-precision%29))
  (|CallParentFunction DeltaSeconds) ; This node is disabled and will not be called.\nDrag off pins to build functionality.
)

(event EventSetupMaterialOwners
  (Rendering|Material|SetMaterial (Variables|Default|GetStaticMesh) 0 (Variables|Default|GetMain%20Power%20Material)))

(event EventOnUpdatePowerFinished
  (params (Forced :type Boolean))
  (CallFunction|UpdatePoweronTarget Forced (Variables|Default|GetTargetActor) false false))

(fn ConstructionScript
  (|CallParentFunction))